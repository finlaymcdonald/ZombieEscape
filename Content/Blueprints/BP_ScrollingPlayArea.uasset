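; BP_ScrollingPlayArea is a conveyor-style play area that spawns obstacles and scrolls them along its local Y axis.
; A self-rescheduling timer spawns one of three random obstacle classes at SpawnPoint, at randomized intervals.
; AddToBelt attaches each obstacle to ScrollParent, keeping its world transform.
; Tick offsets ScrollParent by RunSpeed scaled by delta time, so everything attached moves together.
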(event Custom|AddToBelt
  (params (Actor :type Actor%20Object%20Reference))
  (Transformation|AttachComponentToComponent Actor (Variables|Default|GetScrollParent) "None" "KeepWorld" "KeepWorld" "KeepWorld" true))

(event Custom|SpawnObstacle
  (bind _obstaclespawnintervalrange (Variables|Default|GetObstacleSpawnIntervalRange))
  (bind _returnvalue (Game|SpawnActorfromClass (Utilities|Array|Get(acopy) (Variables|Default|GetObstacleClasses) (Math|Random|RandomInteger 3)) (Transformation|GetWorldTransform (Variables|Default|GetSpawnPoint)) "Undefined" 0 0))
  (CallFunction|AddtoBelt _returnvalue)
  (Utilities|Time|SetTimerbyEvent (delegate Custom|SpawnObstacle) (Math|Random|RandomFloatinRange (.x _obstaclespawnintervalrange) (.y _obstaclespawnintervalrange))))

(event EventBeginPlay
  (bind _obstaclespawnintervalrange (Variables|Default|GetObstacleSpawnIntervalRange))
  (Utilities|Time|SetTimerbyEvent (delegate Custom|SpawnObstacle) (Math|Random|RandomFloatinRange (.x _obstaclespawnintervalrange) (.y _obstaclespawnintervalrange))))

(event Collision|EventActorBeginOverlap
  (params (OtherActor :type Actor%20Object%20Reference)))

(event EventTick
  (params (DeltaSeconds :type Float%20%28single-precision%29))
  (Transformation|AddLocalOffset (Variables|Default|GetScrollParent) (Math|Vector|MakeVector 0.0 (* DeltaSeconds (Variables|Default|GetRunSpeed)) 0.0) false false))

(fn ConstructionScript)