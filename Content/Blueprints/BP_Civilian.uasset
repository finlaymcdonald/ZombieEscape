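; BP_Civilian is a civilian actor that the side-scroller player converts into a new runner, apparently a zombie.
; On BeginPlay its plane gets a random material from the civilian material list.
; When a SideScrollerCharacter overlaps its death collision, a one-time guard fires, the current material is mapped to its zombie counterpart and passed to the character's input manager as a new runner.
; The civilian then destroys itself after a short delay.
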(event OnComponentBeginOverlap(HumanDeathCollision)
  (params (OverlappedComponent :type Primitive%20Component%20Object%20Reference) (OtherActor :type Actor%20Object%20Reference) (OtherComp :type Primitive%20Component%20Object%20Reference) (OtherBodyIndex :type Integer) (bFromSweep :type Boolean) (SweepResult :type Hit%20Result%20Structure%20%28by%20ref%29))
  (bind _asside_scroller_character (Utilities|Casting|CastToSideScrollerCharacter OtherActor))
  (if (not (Variables|Default|GetCollided))
    (Variables|Default|SetCollided true)
    (Default|AddNewRunner (Variables|/Game/SideScrollerBP/Blueprints/SideScrollerCharacter.SideScrollerCharacter_C|GetInputMnaager _asside_scroller_character) (.Value (Utilities|Map|Find (Variables|Default|GetCivToZomMats) (.AsMaterial%20Instance (Utilities|Casting|CastToMaterialInstance (Rendering|Material|GetMaterial (Variables|Default|GetPlane) 0))))))
    (Utilities|FlowControl|Delay 0.2)
    (Actor|DestroyActor)))

(event EventBeginPlay
  (Rendering|Material|SetMaterial (Variables|Default|GetPlane) 0 (Utilities|Array|Get(acopy) (Variables|Default|GetCivMats) (Math|Random|RandomInteger (Utilities|Array|Length (Variables|Default|GetCivMats))))))

(event Collision|EventActorBeginOverlap
  (params (OtherActor :type Actor%20Object%20Reference)))

(event EventTick
  (params (DeltaSeconds :type Float%20%28single-precision%29)))

(fn ConstructionScript)