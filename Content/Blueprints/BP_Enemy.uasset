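; BP_Enemy is a side-scroller enemy that either kills the player character or gets killed and converted into a new runner.
; On BeginPlay its plane gets a random material from EnemyMats.
; ZombieDeathCollision kills the overlapping character unless Collided is set.
; HumanDeathCollision sets that flag, bounces the character, adds a runner using the EnemyToZomMats zombie material, splatters blood, then screams and destroys the enemy after a short delay.
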(event OnComponentBeginOverlap(ZombieDeathCollision)
  (params (OverlappedComponent :type Primitive%20Component%20Object%20Reference) (OtherActor :type Actor%20Object%20Reference) (OtherComp :type Primitive%20Component%20Object%20Reference) (OtherBodyIndex :type Integer) (bFromSweep :type Boolean) (SweepResult :type Hit%20Result%20Structure%20%28by%20ref%29))
  (bind _asside_scroller_character (Utilities|Casting|CastToSideScrollerCharacter OtherActor))
  (if (not (Variables|Default|GetCollided))
    (Effects|SpawnEmitteratLocation "/Game/Effects/PRT_BloodSplatter.PRT_BloodSplatter" (Transformation|GetWorldLocation (Variables|Default|GetParticleLocation)))
    (Default|Kill _asside_scroller_character)))

(event OnComponentBeginOverlap(HumanDeathCollision)
  (params (OverlappedComponent :type Primitive%20Component%20Object%20Reference) (OtherActor :type Actor%20Object%20Reference) (OtherComp :type Primitive%20Component%20Object%20Reference) (OtherBodyIndex :type Integer) (bFromSweep :type Boolean) (SweepResult :type Hit%20Result%20Structure%20%28by%20ref%29))
  (bind _asside_scroller_character (Utilities|Casting|CastToSideScrollerCharacter OtherActor))
  (if (not (Variables|Default|GetCollided))
    (Variables|Default|SetCollided true)
    (Default|Bounce _asside_scroller_character)
    (Default|AddNewRunner (Variables|/Game/SideScrollerBP/Blueprints/SideScrollerCharacter.SideScrollerCharacter_C|GetInputMnaager _asside_scroller_character) (.Value (Utilities|Map|Find (Variables|Default|GetEnemyToZomMats) (.AsMaterial%20Instance (Utilities|Casting|CastToMaterialInstance (Rendering|Material|GetMaterial (Variables|Default|GetPlane) 0))))))
    (Effects|SpawnEmitteratLocation "/Game/Effects/PRT_BloodSplatter.PRT_BloodSplatter" (Transformation|GetWorldLocation (Variables|Default|GetParticleLocation)))
    (Utilities|FlowControl|Delay 0.2)
    (Audio|SpawnSoundatLocation "/Game/Sound/weirderscream__Cue.weirderscream__Cue" "0, 0, 0" "0, 0, 0" 1.0 1.0 0.0 0 0)
    (Actor|DestroyActor)))

(event EventBeginPlay
  (bind _enemymats (Variables|Default|GetEnemyMats))
  (Rendering|Material|SetMaterial (Variables|Default|GetPlane) 0 (Utilities|Array|Get(acopy) _enemymats (Math|Random|RandomInteger (Utilities|Array|Length _enemymats)))))

(event Collision|EventActorBeginOverlap
  (params (OtherActor :type Actor%20Object%20Reference)))

(event EventTick
  (params (DeltaSeconds :type Float%20%28single-precision%29)))

(fn ConstructionScript)